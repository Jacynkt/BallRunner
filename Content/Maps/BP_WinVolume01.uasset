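; Win volume Blueprint that acts as a level exit once the player has collected every Gem.
; When the player overlaps the Werds component, it counts remaining Gem actors and prints a Polish "not all crystals collected" message if any remain.
; Otherwise CompleteLevel opens the hardcoded Level02, but only when the CheckLastLevel flag, read through IsFinalLevel, is true.
; GetCurrentLevelIndex is an empty stub.
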(event OnComponentBeginOverlap(werds)
  (params (OverlappedComponent :type Primitive%20Component%20Object%20Reference) (OtherActor :type Actor%20Object%20Reference) (OtherComp :type Primitive%20Component%20Object%20Reference) (OtherBodyIndex :type Integer) (bFromSweep :type Boolean) (SweepResult :type Hit%20Result%20Structure%20%28by%20ref%29))
  (Utilities|IsPlayer OtherActor
    (:true
      (bind _outactors (Actor|GetAllActorsOfClass "/Game/Maps/Gem.Gem_C"))
      (if (> (Utilities|Array|Length _outactors) 0)
        (Development|PrintString "Nie zebrano wszystkich kryształów")
        (else
          (CallFunction|CompleteLevel))))))

(fn ConstructionScript)

(fn CompleteLevel
  (if (CallFunction|IsFinalLevel)
    (Game|OpenLevel(byName) "Level02")))

(fn IsFinalLevel
  (return (Variables|Default|GetCheckLastLevel)))

(fn GetCurrentLevelIndex)